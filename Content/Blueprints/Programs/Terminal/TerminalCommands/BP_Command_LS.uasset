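; Terminal command Blueprint implementing an LS-style directory listing for the in-game terminal.
; It prints each file of the owning terminal's current directory as name plus extension, then the names of its child directories.
; Hidden files and directories are skipped unless the -a flag is present.
; The command always finishes by reporting success.
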(fn K2onProcessCommand
  (params (CommandToProcess :type String) (bIsRunningAsRoot :type Boolean))
  (Utilities|FlowControl|Sequence
    (:then_0
      (LocalVariables|SetbShowHidden (Class|YetiOSTerminalCommand|HasFlag "-a"))
      (for _array_element (Class|YetiOSDirectoryBase|GetDirectoryFiles (Class|YetiOSTerminalProgram|GetCurrentDirectory (Variables|Default|GetOwningTerminal)))
        (if (.bIsHidden (Utilities|Struct|BreakFileProperties _array_element))
          (if (LocalVariables|GetbShowHidden)
            (Class|YetiOSTerminalCommand|NotifyTerminal (Utilities|Text|FormatText "{Name}{Ext}" (.FileName (Utilities|Struct|BreakFileProperties _array_element)) (.FileExtension (Utilities|Struct|BreakFileProperties _array_element))) "LEVEL_Normal" :!label _label))
          (else
            (goto _label))))
      (for _array_element_2 (Class|YetiOSDirectoryBase|GetAllChildDirectories (Class|YetiOSTerminalProgram|GetCurrentDirectory (Variables|Default|GetOwningTerminal)))
        (LocalVariables|SetLocal_IteratedDirectory _array_element_2)
        (if (Class|YetiOSDirectoryBase|IsHidden (LocalVariables|GetLocal_IteratedDirectory))
          (if (LocalVariables|GetbShowHidden)
            (Class|YetiOSTerminalCommand|NotifyTerminal (Class|YetiOSDirectoryBase|GetDirectoryName (LocalVariables|GetLocal_IteratedDirectory)) "LEVEL_Normal" :!label _label_2))
          (else
            (goto _label_2)))))
    (:then_1
      (Class|YetiOSTerminalCommand|OnSuccess)
      (return true))))