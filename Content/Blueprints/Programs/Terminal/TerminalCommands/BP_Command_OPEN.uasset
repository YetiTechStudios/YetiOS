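; Terminal command OPEN for the in-game terminal, which launches a new program by name.
; It expects exactly one operand, converts it to a name and passes it to OpenNewProgram.
; A wrong operand count or a failed launch sets an error message.
; A sequence then reports through OnSuccess or OnFail, and the process function always returns false regardless of outcome.
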(fn K2onProcessCommand
  (params (CommandToProcess :type String) (bIsRunningAsRoot :type Boolean))
  (bind _commandparameters (Variables|Default|GetCommandParameters))
  (LocalVariables|SetbLocal_Success false)
  (Utilities|FlowControl|Sequence
    (:then_0
      (if (== (Utilities|Array|Length _commandparameters) 1)
        (bind (_outerrormessage _returnvalue) (Class|YetiOSTerminalCommand|OpenNewProgram (Utilities|String|StringToName (Utilities|Array|Get(acopy) _commandparameters))))
        (if _returnvalue
          (LocalVariables|SetbLocal_Success true)
          (else
            (LocalVariables|SetLocal_ErrorMessage (.ErrorException (Utilities|Struct|BreakYetiOsError _outerrormessage)))))
        (else
          (LocalVariables|SetLocal_ErrorMessage (Utilities|Text|FormatText "{TerminalName}: error: {CurrentCommand}: incorrect operands" (Utilities|Text|ToText(String) (Variables|Default|GetTerminalName)) (Utilities|Text|ToText(String) (Variables|Default|GetCurrentCommand)))))))
    (:then_1
      (if (LocalVariables|GetbLocal_Success)
        (Class|YetiOSTerminalCommand|OnSuccess)
        (else
          (Class|YetiOSTerminalCommand|OnFail (Utilities|String|ToString(Text) (LocalVariables|GetLocal_ErrorMessage))))))
    (:then_2
      (return false))))