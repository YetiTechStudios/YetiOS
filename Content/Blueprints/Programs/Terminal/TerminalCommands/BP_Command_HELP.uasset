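; Terminal HELP command that shows usage information for another command in the in-game terminal.
; It takes exactly one parameter and searches the owning terminal's registered commands for a matching main command name.
; On a match it prints that command's description plus a list of its flags, built by a helper from the flag map.
; A missing or extra parameter fails with an error message, while an unknown command fails without setting one.
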(fn K2onProcessCommand
  (params (CommandToProcess :type String) (bIsRunningAsRoot :type Boolean))
  (bind _commandparameters (Variables|Default|GetCommandParameters))
  (bind _returnvalue (Utilities|Array|Length _commandparameters))
  (Utilities|FlowControl|Sequence
    (:then_0
      (Utilities|ArrayHasItems _commandparameters
        (:HasItems
          (if (== _returnvalue 1)
            (LocalVariables|SetLocal_TargetHelpCommand (Utilities|Array|Get(acopy) (Variables|Default|GetCommandParameters)))
            (bind _array_element (Utilities|Array|ForEachLoopwithBreak (Class|YetiOSTerminalProgram|GetAllCommands (Variables|Default|GetOwningTerminal)) :!label _label)
              (:LoopBody
                (if (Utilities|Enum|Equal(Enum) (Class|YetiOSTerminalCommand|GetMainCommand _array_element) (LocalVariables|GetLocal_TargetHelpCommand))
                  (Class|YetiOSTerminalCommand|NotifyTerminal (Utilities|Text|FormatText "Help for command {Command} 
======================== 
{Description} 
{Flags}" (Utilities|Text|ToText(String) (LocalVariables|GetLocal_TargetHelpCommand)) (Utilities|Text|ToText(String) (Class|YetiOSTerminalCommand|GetMainCommandDescription _array_element)) (Utilities|Text|ToText(String) (CallFunction|InternalProcessFlagHelp _array_element))) "LEVEL_Normal")
                  (LocalVariables|SetbLocal_Success true)
                  (goto _label Break))))
            (else
              (LocalVariables|SetbLocal_Success false)
              (LocalVariables|SetLocal_ErrorMessage (Utilities|String|Append (Variables|Default|GetTerminalName) ": error: " (Variables|Default|GetCurrentCommand) (Utilities|String|BuildString(Integer) "" " Found " _returnvalue " params. "))))))
        (:EmptyArray
          (LocalVariables|SetbLocal_Success false)
          (LocalVariables|SetLocal_ErrorMessage (Utilities|String|Append (Variables|Default|GetTerminalName) ": error: " (Variables|Default|GetCurrentCommand) " requires a command to display information.")))))
    (:then_1
      (if (LocalVariables|GetbLocal_Success)
        (Class|YetiOSTerminalCommand|OnSuccess)
        (else
          (Class|YetiOSTerminalCommand|OnFail (LocalVariables|GetLocal_ErrorMessage)))))
    (:then_2
      (return true))))

(fn InternalProcessFlagHelp
  (params (InTargetCommand :type Yeti%20OS%20Terminal%20Command%20Object%20Reference%20%28by%20ref%29))
  (bind _returnvalue (Class|YetiOSTerminalCommand|GetCommandFlags InTargetCommand))
  (Utilities|FlowControl|Sequence
    (:then_0
      (bind _keys (Utilities|Map|Keys _returnvalue))
      (for _array_element _keys
        (LocalVariables|SetLocal_ReturnValue (Utilities|String|Append (LocalVariables|GetLocal_ReturnValue) " 
" _array_element ": " (.Description (Utilities|Struct|BreakYetiOsTerminalCommand (.Value (Utilities|Map|Find _returnvalue _array_element))))))))
    (:then_1
      (return (LocalVariables|GetLocal_ReturnValue)))))