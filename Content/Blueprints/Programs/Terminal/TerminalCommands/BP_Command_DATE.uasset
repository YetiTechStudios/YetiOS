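; Terminal command for the in-game terminal program that prints the current date.
; Overrides the process-command event to format Today as day-month-year, converting the year to text separately, and appends the hour and minute from Now when the -t flag is present.
; Sends the result to the terminal as a normal message and always reports success.
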(fn K2onProcessCommand
  (params (CommandToProcess :type String) (bIsRunningAsRoot :type Boolean))
  (bind _returnvalue (Math|DateTime|Now))
  (bind _returnvalue_2 (Class|KismetMathLibrary|Today))
  (bind (_year _month _day _hour _minute) (Math|DateTime|BreakDateTime _returnvalue))
  (bind (_year_2 _month_2 _day_2) (Math|DateTime|BreakDateTime _returnvalue_2))
  (bind _returnvalue_3 (Utilities|Text|ToText(Integer) _year_2 false false))
  (bind _result (Utilities|Text|FormatText "{Day}-{Month}-{Year}" _day_2 _month_2 _returnvalue_3))
  (Class|YetiOSTerminalCommand|NotifyTerminal (select (Class|YetiOSTerminalCommand|HasFlag "-t") (Utilities|Text|FormatText "{Previous}    {Hour}:{Min}" _result _hour _minute) _result) "LEVEL_Normal")
  (Class|YetiOSTerminalCommand|OnSuccess)
  (return true))