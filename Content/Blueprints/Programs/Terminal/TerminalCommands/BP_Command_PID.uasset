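; Terminal command for the in-game OS that reports process IDs of running programs.
; With -p and one identifier it looks up that program and prints its PID, name and identifier, or builds a not-found or incorrect-operands error.
; Without parameters it chains all running programs into one message, newest iteration first.
; OnSuccess or OnFail follows from LocalSuccess, which the list-all path never sets, so listing ends in OnFail.
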(fn K2onProcessCommand
  (params (CommandToProcess :type String) (bIsRunningAsRoot :type Boolean))
  (bind _owningterminal (Variables|Default|GetOwningTerminal))
  (bind _terminalname (Variables|Default|GetTerminalName))
  (bind _currentcommand (Variables|Default|GetCurrentCommand))
  (bind _owningterminal_2 (Variables|Default|GetOwningTerminal))
  (bind _commandparameters (Variables|Default|GetCommandParameters))
  (bind _returnvalue (Class|YetiOSBaseProgram|GetOwningOS _owningterminal_2))
  (bind _returnvalue_2 (Utilities|Text|ToText(String) _currentcommand))
  (bind _returnvalue_3 (Utilities|Text|ToText(String) _terminalname))
  (bind _returnvalue_4 (Class|YetiOSBaseProgram|GetOwningOS _owningterminal))
  (bind _output (Utilities|Array|Get(acopy) _commandparameters))
  (bind _returnvalue_5 (Utilities|String|StringToName _output))
  (bind _returnvalue_6 (Class|YetiOSCore|GetAllRunningPrograms _returnvalue_4))
  (bind _returnvalue_7 (Class|YetiOSCore|FindRunningProgrambyIdentifier _returnvalue _returnvalue_5))
  (bind _returnvalue_8 (Utilities|GetClass _returnvalue_7))
  (bind (_programname _programidentifier) (Utilities|GetClassDefaults _returnvalue_8))
  (LocalVariables|SetbLocal_Success false)
  (Utilities|FlowControl|Sequence
    (:then_0
      (Utilities|ArrayHasItems (Variables|Default|GetCommandParameters)
        (:HasItems
          (if (== (Utilities|Array|Length _commandparameters) 1)
            (if (Class|YetiOSTerminalCommand|HasFlag "-p")
              (Utilities|IsValid _returnvalue_7
                (:Is%20Valid
                  (LocalVariables|SetbLocal_Success true)
                  (LocalVariables|SetLocal_PidMessage (Utilities|Text|FormatText "PID: {Pid}    -    {ProcessName} ({Identifier})" (Utilities|Text|ToText(Integer) (Class|YetiOSBaseProgram|GetProcessID _returnvalue_7) false false) _programname (Utilities|Text|ToText(Name) _programidentifier)))
                  (Class|YetiOSTerminalCommand|NotifyTerminal (LocalVariables|GetLocal_PidMessage) "LEVEL_Normal" :!label _label))
                (:Is%20Not%20Valid
                  (LocalVariables|SetLocal_ErrorMessage (Utilities|Text|FormatText "{TerminalName}: error: {CurrentCommand}: {Identifier} was not found." _returnvalue_3 _returnvalue_2 (Utilities|Text|ToText(Name) (Utilities|String|StringToName (Utilities|Array|Get(acopy) (Variables|Default|GetCommandParameters))))))))
              (else
                (LocalVariables|SetLocal_ErrorMessage (Utilities|Text|FormatText "{TerminalName}: error: {CurrentCommand}: incorrect operands" _returnvalue_3 _returnvalue_2) :!label _label_2)))
            (else
              (goto _label_2))))
        (:EmptyArray
          (bind _keys (Utilities|Map|Keys _returnvalue_6))
          (for _array_element _keys
            (if (== _array_element 0)
              (LocalVariables|SetLocal_PidMessage (Utilities|Text|FormatText "PID: {Pid}    -    {ProcessName} ({Identifier})" (Utilities|Text|ToText(Integer) _array_element false false) (.ProgramName (Utilities|GetClassDefaults (Utilities|GetClass (.Value (Utilities|Map|Find _returnvalue_6 _array_element))))) (Utilities|Text|ToText(Name) (.ProgramIdentifier (Utilities|GetClassDefaults (Utilities|GetClass (.Value (Utilities|Map|Find _returnvalue_6 _array_element))))))))
              (else
                (LocalVariables|SetLocal_PidMessage (Utilities|Text|FormatText "PID: {Pid}    -    {ProcessName} ({Identifier}) 
{Previous}" (Utilities|Text|ToText(Integer) _array_element false false) (.ProgramName (Utilities|GetClassDefaults (Utilities|GetClass (.Value (Utilities|Map|Find _returnvalue_6 _array_element))))) (Utilities|Text|ToText(Name) (.ProgramIdentifier (Utilities|GetClassDefaults (Utilities|GetClass (.Value (Utilities|Map|Find _returnvalue_6 _array_element)))))) (LocalVariables|GetLocal_PidMessage))))))
          (goto _label))))
    (:then_1
      (if (LocalVariables|GetbLocal_Success)
        (Class|YetiOSTerminalCommand|OnSuccess)
        (else
          (Class|YetiOSTerminalCommand|OnFail (Utilities|String|ToString(Text) (LocalVariables|GetLocal_ErrorMessage))))))
    (:then_2
      (return true))))