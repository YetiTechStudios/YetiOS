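; Terminal command that implements TOUCH for the in-game terminal, creating files in the owning terminal's current directory.
; It loops over the parameters, splitting each on dots to derive name and extension, then creates a deletable, movable file without forcing.
; The -h flag hides files and -v reports each creation.
; Individual creation errors are printed, but the command fails only when no parameters are given.
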(fn K2onProcessCommand
  (params (CommandToProcess :type String) (bIsRunningAsRoot :type Boolean))
  (bind _currentcommand (Variables|Default|GetCurrentCommand))
  (bind _commandparameters (Variables|Default|GetCommandParameters))
  (LocalVariables|SetLocal_Command CommandToProcess)
  (Utilities|FlowControl|Sequence
    (:then_0
      (Utilities|ArrayHasItems _commandparameters
        (:HasItems
          (bind _output_get (LocalVariables|SetLocal_TotalParams (Utilities|Array|Length _commandparameters)))
          (LocalVariables|SetbLocal_Success true)
          (LocalVariables|SetbLocal_HasVerboseFlag (Class|YetiOSTerminalCommand|HasFlag "-v"))
          (for _index (range 0 (- _output_get 1))
            (LocalVariables|SetLocal_IteratedCommand (Utilities|Array|Get(acopy) (Variables|Default|GetCommandParameters) _index))
            (Utilities|FlowControl|Sequence
              (:then_0
                (Utilities|ArrayHasItems (Utilities|String|ParseIntoArray (LocalVariables|GetLocal_IteratedCommand) ".")
                  (:HasItems
                    (LocalVariables|SetLocal_FileExtension (Utilities|Text|FormatText ".{Extension}" (Utilities|Text|ToText(String) (Utilities|Array|Get(acopy) (Utilities|String|ParseIntoArray (LocalVariables|GetLocal_IteratedCommand) ".") (Utilities|Array|LastIndex (Utilities|String|ParseIntoArray (LocalVariables|GetLocal_IteratedCommand) "."))))))
                    (LocalVariables|SetLocal_IteratedFileName (Utilities|Text|ToText(String) (Utilities|String|Left (LocalVariables|GetLocal_IteratedCommand) (- (- (Utilities|String|Len (LocalVariables|GetLocal_IteratedCommand)) (Utilities|String|Len (Utilities|Array|Get(acopy) (Utilities|String|ParseIntoArray (LocalVariables|GetLocal_IteratedCommand) ".") (Utilities|Array|LastIndex (Utilities|String|ParseIntoArray (LocalVariables|GetLocal_IteratedCommand) "."))))) 1)))))
                  (:EmptyArray
                    (LocalVariables|SetLocal_FileExtension ".file")
                    (LocalVariables|SetLocal_IteratedFileName (Utilities|Text|ToText(String) (LocalVariables|GetLocal_IteratedCommand))))))
              (:then_1
                (bind (_outerrormessage _returnvalue) (Class|YetiOSDirectoryBase|CreateNewFile (Class|YetiOSTerminalProgram|GetCurrentDirectory (Variables|Default|GetOwningTerminal)) (Utilities|Struct|MakeFileProperties (LocalVariables|GetLocal_IteratedFileName) "" (LocalVariables|GetLocal_FileExtension) "/YetiOS/YetiOS/DefaultIcons/T_UI_FileIcon.T_UI_FileIcon" (Class|YetiOSTerminalCommand|HasFlag "-h") true true) false))
                (if _returnvalue
                  (if (LocalVariables|GetbLocal_HasVerboseFlag)
                    (Class|YetiOSTerminalCommand|NotifyTerminal (Utilities|Text|FormatText "{Com}: created file '{FileName}'" (Utilities|Text|ToText(String) (Variables|Default|GetCurrentCommand)) (LocalVariables|GetLocal_IteratedFileName)) "LEVEL_Normal"))
                  (else
                    (Class|YetiOSTerminalCommand|NotifyTerminal (.ErrorDetailedException (Utilities|Struct|BreakYetiOsError _outerrormessage)) "LEVEL_Error")))))))
        (:EmptyArray
          (LocalVariables|SetbLocal_Success false)
          (LocalVariables|SetLocal_ErrorMessage (Utilities|String|Append (Variables|Default|GetTerminalName) ": error: " _currentcommand " requires file name. 
Try 'help -" _currentcommand "' for more info.")))))
    (:then_1
      (if (LocalVariables|GetbLocal_Success)
        (Class|YetiOSTerminalCommand|OnSuccess)
        (else
          (Class|YetiOSTerminalCommand|OnFail (LocalVariables|GetLocal_ErrorMessage)))))
    (:then_2
      (return true))))