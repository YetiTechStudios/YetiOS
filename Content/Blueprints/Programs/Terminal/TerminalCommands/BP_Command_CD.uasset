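; BP_Command_CD is the "cd" command for the in-game terminal program, changing the owning terminal's current path.
; Processing expects exactly one parameter, which it passes to the terminal's ChangeCurrentPath, then reports success or a no-such-directory failure.
; A wrong parameter count also fails with an error message, and the handler returns true in every case.
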(fn K2onProcessCommand
  (params (CommandToProcess :type String) (bIsRunningAsRoot :type Boolean))
  (bind _commandparameters (Variables|Default|GetCommandParameters))
  (bind _output (Utilities|Array|Get(acopy) _commandparameters))
  (Utilities|FlowControl|Sequence
    (:then_0
      (bind _output_get (LocalVariables|SetLocal_FlagCount (Utilities|Array|Length (Variables|Default|GetCommandParameters))))
      (if (== _output_get 1)
        (bind _returnvalue (Class|YetiOSTerminalProgram|ChangeCurrentPath (Variables|Default|GetOwningTerminal) _output))
        (if _returnvalue
          (Class|YetiOSTerminalCommand|OnSuccess)
          (else
            (Class|YetiOSTerminalCommand|OnFail (Utilities|String|Append (Variables|Default|GetTerminalName) ": error: " _output (Variables|Default|GetCurrentCommand) ": No such file or directory"))))
        (else
          (Class|YetiOSTerminalCommand|OnFail (Utilities|String|BuildString(Integer) "" (Utilities|String|Append (Variables|Default|GetTerminalName) ": error: Found ") (LocalVariables|GetLocal_FlagCount) " flags. ")))))
    (:then_1
      (return true))))