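; Terminal command PROGRAMS, which lists the programs on the owning terminal's OS.
; With the -all flag, it first prints repository programs as not installed, reading names from class defaults, or reports an error if no valid repository exists.
; It then always prints the currently installed programs and reports success, even after a repository error.
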(fn K2onProcessCommand
  (params (CommandToProcess :type String) (bIsRunningAsRoot :type Boolean))
  (Utilities|FlowControl|Sequence
    (:then_0
      (LocalVariables|SetLocal_OS (Class|YetiOSBaseProgram|GetOwningOS (Variables|Default|GetOwningTerminal)))
      (if (Class|YetiOSTerminalCommand|HasFlag "-all")
        (bind (_outprograms _returnvalue) (Class|YetiOSCore|GetAllProgramsfromRepositoryLibrary (LocalVariables|GetLocal_OS)))
        (if _returnvalue
          (Class|YetiOSTerminalCommand|NotifyTerminal (Utilities|Text|FormatText "=====FROM REPOSITORY======") "LEVEL_Normal")
          (for _array_element _outprograms
            (Class|YetiOSTerminalCommand|NotifyTerminal (Utilities|Text|FormatText "{ProgramName} - Not Installed" (Utilities|GetClassDefaults _array_element)) "LEVEL_Normal"))
          (else
            (Class|YetiOSTerminalCommand|NotifyTerminal (Utilities|Text|FormatText "Valid repository was not found on this OS.") "LEVEL_Error")))))
    (:then_1
      (Class|YetiOSTerminalCommand|NotifyTerminal (Utilities|Text|FormatText "=====CURRENTLY INSTALLED PROGRAMS======") "LEVEL_Normal")
      (for _array_element_2 (Class|YetiOSCore|GetInstalledPrograms (LocalVariables|GetLocal_OS))
        (Class|YetiOSTerminalCommand|NotifyTerminal (Utilities|Text|FormatText "{ProgramName} - Installed" (Variables|/Script/YetiOS.YetiOS_BaseProgram|GetProgramName _array_element_2)) "LEVEL_Normal")))
    (:then_2
      (Class|YetiOSTerminalCommand|OnSuccess)
      (return true))))