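; Terminal command ADDUSER for the in-game Yeti OS, which creates a new user account when processed as root.
; It takes a username and an optional password, rejecting empty or excess operands, and passes them with a default icon to the owning OS's AddNewUser.
; It notifies the terminal on creation, then reports success, or failure with a formatted error, and always returns true.
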(fn K2onProcessCommandasRoot
  (params (CommandToProcess :type String))
  (bind _currentcommand (Variables|Default|GetCurrentCommand))
  (bind _commandparameters (Variables|Default|GetCommandParameters))
  (bind _output (Utilities|Array|Get(acopy) _commandparameters))
  (bind _returnvalue (Utilities|Text|ToText(String) _output))
  (LocalVariables|SetbLocal_Success false)
  (Utilities|FlowControl|Sequence
    (:then_0
      (if (> (Utilities|Array|Length (Variables|Default|GetCommandParameters)) 2)
        (LocalVariables|SetLocal_ErrorMessage (Utilities|String|Append (Variables|Default|GetTerminalName) ": error: " _currentcommand ": incorrect operands." " 
" "Try '" _currentcommand " --help' for more information.") :!label _label)
        (else
          (Utilities|ArrayHasItems (Variables|Default|GetCommandParameters)
            (:HasItems
              (bind (_outerrormessage _returnvalue_2) (Class|YetiOSCore|AddNewUser (Class|YetiOSBaseProgram|GetOwningOS (Variables|Default|GetOwningTerminal)) (Utilities|Struct|MakeYetiOsUser _returnvalue (select (Utilities|Array|IsValidIndex (Variables|Default|GetCommandParameters) 1) (Utilities|Text|ToText(String) (Utilities|Array|Get(acopy) _commandparameters 1)) "") "/YetiOS/YetiOS/Material/M_UI_DefaultUserIcon.M_UI_DefaultUserIcon")))
              (bind _output_get (LocalVariables|SetbLocal_Success _returnvalue_2))
              (if _output_get
                (Class|YetiOSTerminalCommand|NotifyTerminal (Utilities|Text|FormatText "New user created: {User}" _returnvalue) "LEVEL_Normal")
                (else
                  (LocalVariables|SetLocal_ErrorMessage (Utilities|String|Append (Variables|Default|GetTerminalName) ": error: " (Variables|Default|GetCurrentCommand) ": " (Utilities|String|ToString(Text) (.ErrorCode (Utilities|Struct|BreakYetiOsError _outerrormessage))) ".  
" (Utilities|String|ToString(Text) (.ErrorException (Utilities|Struct|BreakYetiOsError _outerrormessage))))))))
            (:EmptyArray
              (goto _label))))))
    (:then_1
      (if (LocalVariables|GetbLocal_Success)
        (Class|YetiOSTerminalCommand|OnSuccess)
        (else
          (Class|YetiOSTerminalCommand|OnFail (LocalVariables|GetLocal_ErrorMessage)))))
    (:then_2
      (return true))))