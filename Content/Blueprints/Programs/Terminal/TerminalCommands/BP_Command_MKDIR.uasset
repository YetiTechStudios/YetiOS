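; Terminal command Blueprint for mkdir, which creates folders in the in-game terminal's current directory.
; It checks for parameters and folder-creation permission, then creates a child directory from the owning OS's template for each name, with flags for hidden and verbose output.
; Creation errors go straight to the terminal, while OnSuccess or OnFail fires once at the end, reflecting the last attempt when several names are given.
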(fn K2onProcessCommand
  (params (CommandToProcess :type String) (bIsRunningAsRoot :type Boolean))
  (bind _commandparameters (Variables|Default|GetCommandParameters))
  (bind _currentcommand (Variables|Default|GetCurrentCommand))
  (LocalVariables|SetLocal_Command CommandToProcess)
  (Utilities|FlowControl|Sequence
    (:then_0
      (bind _output_get (LocalVariables|SetLocal_TotalParams (Utilities|Array|Length _commandparameters)))
      (if (>= _output_get 1)
        (bind _output_get_2 (LocalVariables|SetLocal_CurrentDirectory (Class|YetiOSTerminalProgram|GetCurrentDirectory (Variables|Default|GetOwningTerminal))))
        (if (Class|YetiOSDirectoryBase|CanCreateNewFolder _output_get_2)
          (LocalVariables|SetLocal_DirectoryName (Utilities|Text|ToText(String) (Utilities|Array|Get(acopy) _commandparameters)))
          (if (== (LocalVariables|GetLocal_TotalParams) 1)
            (bind (_outerrormessage _returnvalue) (Class|YetiOSDirectoryBase|CreateChildDirectory (LocalVariables|GetLocal_CurrentDirectory) (Class|YetiOSCore|GetTemplateDirectory (Class|YetiOSBaseProgram|GetOwningOS (Variables|Default|GetOwningTerminal))) (LocalVariables|GetLocal_DirectoryName) (Class|YetiOSTerminalCommand|HasFlag "-h") :!label _label))
            (Utilities|FlowControl|Sequence
              (:then_0
                (if (not (Utilities|Text|TextIsEmpty (.ErrorCode (Utilities|Struct|BreakYetiOsError _outerrormessage))))
                  (Class|YetiOSTerminalCommand|NotifyTerminal (.ErrorException (Utilities|Struct|BreakYetiOsError _outerrormessage)) "LEVEL_Error")))
              (:then_1
                (Utilities|IsValid _returnvalue
                  (:Is%20Valid
                    (LocalVariables|SetbLocal_Success true)
                    (if (Class|YetiOSTerminalCommand|HasFlag "-v")
                      (Class|YetiOSTerminalCommand|NotifyTerminal (Utilities|Text|FormatText "{Com}: created directory '{DirName}'" (Utilities|Text|ToText(String) (Variables|Default|GetCurrentCommand)) (LocalVariables|GetLocal_DirectoryName)) "LEVEL_Normal")))
                  (:Is%20Not%20Valid
                    (LocalVariables|SetbLocal_Success false)))))
            (else
              (for _index (range 0 (- (LocalVariables|GetLocal_TotalParams) 1))
                (LocalVariables|SetLocal_DirectoryName (Utilities|Text|ToText(String) (Utilities|Array|Get(acopy) (Variables|Default|GetCommandParameters) _index)))
                (goto _label))))
          (else
            (LocalVariables|SetLocal_ErrorMessage (Utilities|String|Append (Variables|Default|GetTerminalName) ": error: " (Variables|Default|GetCurrentCommand) ": cannot create directory '" (Utilities|Array|Get(acopy) (Variables|Default|GetCommandParameters)) "': Permission denied."))
            (LocalVariables|SetbLocal_Success false)))
        (else
          (LocalVariables|SetLocal_ErrorMessage (Utilities|String|Append (Variables|Default|GetTerminalName) ": error: " _currentcommand ": incorrect operands" " 
" "Try '" _currentcommand " --help' for more information."))
          (LocalVariables|SetbLocal_Success false))))
    (:then_1
      (if (LocalVariables|GetbLocal_Success)
        (Class|YetiOSTerminalCommand|OnSuccess)
        (else
          (Class|YetiOSTerminalCommand|OnFail (LocalVariables|GetLocal_ErrorMessage)))))
    (:then_2
      (return true))))