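; Terminal command that imitates apt-get in the in-game terminal, installing programs from packages on the terminal's owning OS.
; When processed as root, it queues the lowercased parameters other than "install", prints status lines and fails without a package repository.
; It asks for confirmation unless given -y, then starts a short timer before continuing.
; The install function reports each result, succeeding if at least one program installs.
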(event Custom|PromptUserToContinue
  (if (Class|YetiOSTerminalCommand|HasFlag "-y")
    (Class|YetiOSTerminalCommand|OnContinueExecution)
    (else
      (Class|YetiOSTerminalProgram|PromptforUserContinueInput (Variables|Default|GetOwningTerminal)))))

(event EventOnContinueExecution
  (Utilities|ArrayHasItems (Variables|Default|GetProgramsToInstall)
    (:HasItems
      (Utilities|Time|SetTimerbyEvent (EventDispatchers|CreateEvent :!event InternalInstallPrograms) 1.2))
    (:EmptyArray
      (Class|YetiOSTerminalCommand|OnFail "No programs found."))))

(fn K2onProcessCommandasRoot
  (params (CommandToProcess :type String))
  (for _array_element (Variables|Default|GetCommandParameters)
    (if (Utilities|Enum|NotEqual(Enum) (Utilities|String|ToLower _array_element) "install")
      (Utilities|Array|Add (Variables|Default|GetProgramsToInstall) (Utilities|String|ToLower _array_element))))
  (Utilities|FlowControl|Sequence
    (:then_0
      (LocalVariables|SetbLocal_HasPackageRepo (Class|YetiOSTerminalProgram|HasPackageRepo (Variables|Default|GetOwningTerminal)))
      (Class|YetiOSTerminalCommand|NotifyTerminal (Utilities|Text|FormatText "Reading package list...{State}" (select (LocalVariables|GetbLocal_HasPackageRepo) (Utilities|Text|MakeLiteralText "done") (Utilities|Text|MakeLiteralText "fail"))) (select (LocalVariables|GetbLocal_HasPackageRepo) "LEVEL_Normal" "LEVEL_Error"))
      (Class|YetiOSTerminalCommand|NotifyTerminal (Utilities|Text|MakeLiteralText "Building dependecy tree") "LEVEL_Normal")
      (Class|YetiOSTerminalCommand|NotifyTerminal (Utilities|Text|MakeLiteralText "Reading state information...done") "LEVEL_Normal"))
    (:then_1
      (if (LocalVariables|GetbLocal_HasPackageRepo)
        (CallFunction|PromptUsertoContinue)
        (else
          (Class|YetiOSTerminalCommand|OnFail "package repository not found."))))
    (:then_2
      (return true))))

(fn InternalInstallPrograms
  (bind _failedpackages (Variables|Default|GetFailedPackages))
  (for _array_element (Variables|Default|GetProgramsToInstall)
    (bind (_outerrormessage _outiconwidget _returnvalue) (Class|YetiOSCore|InstallProgramfromPackage (Class|YetiOSBaseProgram|GetOwningOS (Variables|Default|GetOwningTerminal)) _array_element))
    (Utilities|IsValid _returnvalue
      (:Is%20Valid
        (Class|YetiOSTerminalCommand|NotifyTerminal (Utilities|Text|FormatText "'{Program}' installed successfully." (Variables|/Script/YetiOS.YetiOS_BaseProgram|GetProgramName _returnvalue)) "LEVEL_Normal")
        (LocalVariables|SetbLocal_AtleastOneProgramInstalled true))
      (:Is%20Not%20Valid
        (Utilities|Map|Add (Variables|Default|GetFailedPackages) _array_element _outerrormessage))))
  (Utilities|FlowControl|Sequence
    (:then_0
      (bind _keys (Utilities|Map|Keys _failedpackages))
      (Utilities|ArrayHasItems _keys
        (:HasItems
          (for _array_element_2 _keys
            (Class|YetiOSTerminalCommand|NotifyTerminal (Utilities|Text|FormatText "Failed to install '{Package}': {Exception}" (Utilities|Text|ToText(String) _array_element_2) (.ErrorException (Utilities|Struct|BreakYetiOsError (.Value (Utilities|Map|Find _failedpackages _array_element_2))))) "LEVEL_Error")))))
    (:then_1
      (if (LocalVariables|GetbLocal_AtleastOneProgramInstalled)
        (Class|YetiOSTerminalCommand|OnSuccess)
        (else
          (Class|YetiOSTerminalCommand|OnFail "package(s) failed to install."))))))