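; BP_Settings_Browser is the saved settings object for the in-game web browser program.
; On PreSave it pulls the home URL and startup option from the owning program's WBP_WebBrowser widget.
; It clears the stored open URLs and refills them from the widget only for one specific startup option.
; Getter functions expose the three stored values.
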(event EventPreSave
  (bind _returnvalue (Class|YetiOSProgramSettings|GetOwningProgram))
  (bind _returnvalue_2 (Class|YetiOSBaseProgram|GetProgramWidget _returnvalue))
  (bind _aswbp_web_browser (Utilities|Casting|CastToWBP_WebBrowser _returnvalue_2))
  (Utilities|Array|Clear (Variables|Default|GetOpenURLs))
  (Variables|Default|SetHomeURL (Default|GetHomeURL _aswbp_web_browser))
  (bind _output_get (Variables|Default|SetStartupOption (Default|GetStartupOption _aswbp_web_browser)))
  (if (Utilities|Enum|Equal(Enum) _output_get "NewEnumerator1")
    (Variables|Default|SetOpenURLs (Default|GetOpenURLs _aswbp_web_browser))))

(fn GetStartupOption
  (return (Variables|Default|GetStartupOption)))

(fn GetOpenURLs
  (return (Variables|Default|GetOpenURLs)))

(fn GetHomeURL
  (return (Variables|Default|GetHomeURL)))